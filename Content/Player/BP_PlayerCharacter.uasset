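; Player character Blueprint that handles basic walking and mouse look through axis input events.
; MoveForward and MoveRight feed movement input along the Camera component's forward and right vectors, so walking follows the view direction.
; Mouse axes drive controller yaw and negated pitch, scaled by frame delta time and a MouseSensitivity variable.
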(event Input|AxisEvents|InputAxisMoveForward
  (params (AxisValue :type Float%20%28single-precision%29))
  ;[0 0 0] Walking
  (Pawn|Input|AddMovementInput (Math|Vector|GetForwardVector (Variables|Default|GetCamera)) AxisValue false))

(event Input|AxisEvents|InputAxisMoveRight
  (params (AxisValue :type Float%20%28single-precision%29))
  ;[0 0 0] Walking
  (Pawn|Input|AddMovementInput (Math|Vector|GetRightVector (Variables|Default|GetCamera)) AxisValue false))

(event Input|AxisEvents|InputAxisMouseUp
  (params (AxisValue :type Float%20%28single-precision%29))
  ;[0 0 0] Camera Look
  (Pawn|Input|AddControllerPitchInput (* (* (* AxisValue (Utilities|Time|GetWorldDeltaSeconds)) (Variables|Default|GetMouseSensitivity)) -1.0)))

(event Input|AxisEvents|InputAxisMouseRight
  (params (AxisValue :type Float%20%28single-precision%29))
  ;[0 0 0] Camera Look
  (Pawn|Input|AddControllerYawInput (* (* AxisValue (Utilities|Time|GetWorldDeltaSeconds)) (Variables|Default|GetMouseSensitivity))))

(fn ConstructionScript)