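; GM_Test, apparently a test game mode, builds and rebuilds a set of random walls at marked spawn points.
; On BeginPlay it caches all BP_SpawnPoint actors and binds SpawnWalls to the player's successful door interaction event, then runs it once.
; SpawnWalls destroys tracked walls, removing them mid-loop, then spawns a BP_RandomWall at each point.
; Each point's WallPosition sets a fixed yaw, except Start, which keeps its own rotation.
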(event Custom|Spawn%20Walls
  (for _array_element (Variables|Default|GetSpawnedWalls)
    (Utilities|IsValid _array_element
      (:Is%20Valid
        (Actor|DestroyActor _array_element)
        (Utilities|Array|RemoveItem (Variables|Default|GetSpawnedWalls) _array_element))))
  (for _array_element_2 (Variables|Default|GetWallSpawns)
    (switch Utilities|FlowControl|Switch|SwitchonE_WallPosition (Variables|/Game/_ProjectCUM/Blueprints/BP_SpawnPoint.BP_SpawnPoint_C|GetWallPosition _array_element_2)
      (:NewEnumerator0
        (bind _returnvalue (Game|SpawnActorfromClass "/Game/_ProjectCUM/Blueprints/BP_RandomWall.BP_RandomWall_C" (Math|Transform|MakeTransform (.location (Transformation|GetActorTransform _array_element_2)) (Math|Rotator|MakeRotator (.roll (.rotation (Transformation|GetActorTransform _array_element_2))) (.pitch (.rotation (Transformation|GetActorTransform _array_element_2))) (.yaw (.rotation (Transformation|GetActorTransform _array_element_2)))) (.scale (Transformation|GetActorTransform _array_element_2))) "AdjustIfPossibleButAlwaysSpawn" 0 0))
        (Utilities|Array|Add (Variables|Default|GetSpawnedWalls) _returnvalue))
      (:NewEnumerator1
        (Game|SpawnActorfromClass "/Game/_ProjectCUM/Blueprints/BP_RandomWall.BP_RandomWall_C" (Math|Transform|MakeTransform (.location (Transformation|GetActorTransform _array_element_2)) (Math|Rotator|MakeRotator (.roll (.rotation (Transformation|GetActorTransform _array_element_2))) (.pitch (.rotation (Transformation|GetActorTransform _array_element_2))) -9e+01) (.scale (Transformation|GetActorTransform _array_element_2))) "AdjustIfPossibleButAlwaysSpawn" 0 0)
        (Utilities|Array|Add (Variables|Default|GetSpawnedWalls) 0))
      (:NewEnumerator2
        (Game|SpawnActorfromClass "/Game/_ProjectCUM/Blueprints/BP_RandomWall.BP_RandomWall_C" (Math|Transform|MakeTransform (.location (Transformation|GetActorTransform _array_element_2)) (Math|Rotator|MakeRotator (.roll (.rotation (Transformation|GetActorTransform _array_element_2))) (.pitch (.rotation (Transformation|GetActorTransform _array_element_2))) 9e+01) (.scale (Transformation|GetActorTransform _array_element_2))) "AdjustIfPossibleButAlwaysSpawn" 0 0)
        (Utilities|Array|Add (Variables|Default|GetSpawnedWalls) 0))
      (:NewEnumerator3
        (Game|SpawnActorfromClass "/Game/_ProjectCUM/Blueprints/BP_RandomWall.BP_RandomWall_C" (Math|Transform|MakeTransform (.location (Transformation|GetActorTransform _array_element_2)) (Math|Rotator|MakeRotator (.roll (.rotation (Transformation|GetActorTransform _array_element_2))) (.pitch (.rotation (Transformation|GetActorTransform _array_element_2))) 1.8e+02) (.scale (Transformation|GetActorTransform _array_element_2))) "AdjustIfPossibleButAlwaysSpawn" 0 0)
        (Utilities|Array|Add (Variables|Default|GetSpawnedWalls) 0)))))

(event EventBeginPlay
  (bind _outactors (Actor|GetAllActorsOfClass "/Game/_ProjectCUM/Blueprints/BP_SpawnPoint.BP_SpawnPoint_C"))
  (Variables|Default|SetWallSpawns _outactors)
  (bind _asbp_player_character (Utilities|Casting|CastToBP_PlayerCharacter (Game|Player|GetPlayerPawn 0)))
  (bind _output_get (Variables|Default|SetPawnRef _asbp_player_character))
  (EventDispatchers|BindEventtoOnSuccessfulDoorInteraction _output_get (delegate Custom|Spawn%20Walls))
  (CallFunction|SpawnWalls))

(fn ConstructionScript)