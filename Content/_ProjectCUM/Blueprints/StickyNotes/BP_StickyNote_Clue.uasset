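; BP_StickyNote_Clue is a sticky note that displays either a random clue or random gibberish through a widget component.
; On BeginPlay it caches the WBP_StickyNote widget reference and randomizes the note's background color.
; RandomizeNoteText takes an IsClue flag and passes the clue or gibberish list to the widget, which handles the text randomization; this Blueprint never calls that event itself.
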(event Custom|Randomize%20Background%20Color
  (Default|RandomizeColor (Variables|Default|GetStickyNoteWidgetRef)))

(event Custom|Randomize%20Note%20Text
  (params (IsClue :type Boolean))
  (if IsClue
    (Default|RandomizeText (Variables|Default|GetStickyNoteWidgetRef) (Variables|Default|GetListOfClues))
    (else
      (Default|RandomizeText (Variables|Default|GetStickyNoteWidgetRef) (Variables|Default|GetListOfGibberish)))))

(event EventBeginPlay
  (bind _aswbp_sticky_note (Utilities|Casting|CastToWBP_StickyNote (UserInterface|GetWidget (Variables|Default|GetWidget))))
  (Variables|Default|SetStickyNoteWidgetRef _aswbp_sticky_note)
  (CallFunction|RandomizeBackgroundColor))

(fn ConstructionScript)