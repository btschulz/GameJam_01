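; BP_Door is a door actor that shows an interaction widget when the player character is nearby and flags that the player can use the door.
; InteractTrigger overlaps toggle the widget's visibility, a billboard flag and CanUseDoor on the cached BP_PlayerCharacter.
; While the flag is set, Tick rotates the widget to face the player pawn's location.
; The door itself has no opening logic.
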(event OnComponentBeginOverlap(InteractTrigger)
  (params (OverlappedComponent :type Primitive%20Component%20Object%20Reference) (OtherActor :type Actor%20Object%20Reference) (OtherComp :type Primitive%20Component%20Object%20Reference) (OtherBodyIndex :type Integer) (bFromSweep :type Boolean) (SweepResult :type Hit%20Result%20Structure%20%28by%20ref%29))
  (Utilities|Casting|CastToBP_PlayerCharacter OtherActor)
  (Rendering|SetVisibility (Variables|Default|GetWidget) true false)
  (Variables|Default|SetBillboardWidget true)
  (Variables|/Game/_ProjectCUM/Player/BP_PlayerCharacter.BP_PlayerCharacter_C|SetCanUseDoor (Variables|Default|GetPawnRef) true))

(event OnComponentEndOverlap(InteractTrigger)
  (params (OverlappedComponent :type Primitive%20Component%20Object%20Reference) (OtherActor :type Actor%20Object%20Reference) (OtherComp :type Primitive%20Component%20Object%20Reference) (OtherBodyIndex :type Integer))
  (Utilities|Casting|CastToBP_PlayerCharacter OtherActor)
  (Rendering|SetVisibility (Variables|Default|GetWidget) false false)
  (Variables|Default|SetBillboardWidget false)
  (Variables|/Game/_ProjectCUM/Player/BP_PlayerCharacter.BP_PlayerCharacter_C|SetCanUseDoor (Variables|Default|GetPawnRef) false))

(event EventTick
  (params (DeltaSeconds :type Float%20%28single-precision%29))
  (bind _widget (Variables|Default|GetWidget))
  (if (Variables|Default|GetBillboardWidget)
    (Transformation|SetWorldRotation _widget (Math|Rotator|FindLookatRotation (Transformation|GetWorldLocation _widget) (Transformation|GetActorLocation (Variables|Default|GetPawnRef))) false false)))

(event EventBeginPlay
  (bind _asbp_player_character (Utilities|Casting|CastToBP_PlayerCharacter (Game|Player|GetPlayerPawn 0)))
  (Variables|Default|SetPawnRef _asbp_player_character)
  (Rendering|SetCastShadow (Variables|Default|GetWidget) false))

(fn ConstructionScript)